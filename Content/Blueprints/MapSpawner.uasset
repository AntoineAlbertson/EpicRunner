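; MapSpawner endlessly extends a side-scroller level along X by spawning BaseForest tile maps ahead of the 2DSideScrollerCharacter.
; BeginPlay lays three starting segments, then caches the first character found.
; Each Tick spawns another segment whenever the next spawn point is less than a fixed distance ahead of the character.
; SpawnNewMap creates a scaled PaperTileMapActor, advances SpawnLocation by a fixed step and assigns the tile map; no segments are removed.
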(event EventBeginPlay
  (CallFunction|SpawnNewMap "/Game/GraphicRessources/Tilemaps/BaseForest.BaseForest")
  (CallFunction|SpawnNewMap "/Game/GraphicRessources/Tilemaps/BaseForest.BaseForest")
  (CallFunction|SpawnNewMap "/Game/GraphicRessources/Tilemaps/BaseForest.BaseForest")
  (bind _outactors (Actor|GetAllActorsOfClass "/Game/2DSideScrollerBP/Blueprints/2DSideScrollerCharacter.2DSideScrollerCharacter_C"))
  (Variables|Default|SetCharacter (Utilities|Array|Get(acopy) _outactors)))

(event Collision|EventActorBeginOverlap
  (params (OtherActor :type Actor%20Object%20Reference)))

(event EventTick
  (params (DeltaSeconds :type Float%20%28single-precision%29))
  (if (< (- (.x (Variables|Default|GetSpawnLocation)) (.x (Transformation|GetActorLocation (Variables|Default|GetCharacter)))) 3e+03)
    (CallFunction|SpawnNewMap "/Game/GraphicRessources/Tilemaps/BaseForest.BaseForest")))

(fn ConstructionScript)

(fn UpSpawnLocation
  (Variables|Default|SetSpawnLocation (+ (Variables|Default|GetSpawnLocation) "1280.000000, 0, 0")))

(fn SpawnNewMap
  (params (SpawnedMap :type Paper%20Tile%20Map%20Object%20Reference))
  (bind _returnvalue (Game|SpawnActorfromClass "/Script/Paper2D.PaperTileMapActor" (Math|Transform|MakeTransform (Variables|Default|GetSpawnLocation) "0, 0, 0" (Variables|Default|GetBaseMapScale)) "Undefined" 0 0))
  (CallFunction|UpSpawnLocation)
  (Class|PaperTileMapComponent|SetTileMap (Variables|/Script/Paper2D.PaperTileMapActor|GetRenderComponent _returnvalue) SpawnedMap))