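; FollowingCamera is a side-scroller actor that tracks the player along the X axis and destroys actors that touch its Box.
; BeginPlay caches the first 2DSideScrollerCharacter found in the level.
; Each Tick moves the actor to a fixed X offset from that character, keeping its own Y and Z.
; The Box overlap destroys any entering actor without filtering, so it acts as a moving kill volume.
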(event OnComponentBeginOverlap(Box)
  (params (OverlappedComponent :type Primitive%20Component%20Object%20Reference) (OtherActor :type Actor%20Object%20Reference) (OtherComp :type Primitive%20Component%20Object%20Reference) (OtherBodyIndex :type Integer) (bFromSweep :type Boolean) (SweepResult :type Hit%20Result%20Structure%20%28by%20ref%29))
  (Actor|DestroyActor OtherActor))

(event EventBeginPlay
  (bind _outactors (Actor|GetAllActorsOfClass "/Game/2DSideScrollerBP/Blueprints/2DSideScrollerCharacter.2DSideScrollerCharacter_C"))
  (Variables|Default|SetPlayerRef (Utilities|Array|Get(acopy) _outactors)))

(event Collision|EventActorBeginOverlap
  (params (OtherActor :type Actor%20Object%20Reference)))

(event EventTick
  (params (DeltaSeconds :type Float%20%28single-precision%29))
  (bind _returnvalue (Transformation|GetActorLocation))
  (Transformation|SetActorLocation (Math|Vector|MakeVector (+ (.x (Transformation|GetActorLocation (Variables|Default|GetPlayerRef))) 8e+02) (.y _returnvalue) (.z _returnvalue)) false false))

(fn ConstructionScript)